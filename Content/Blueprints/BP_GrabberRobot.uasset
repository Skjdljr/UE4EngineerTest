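; BP_GrabberRobot is the "Grabber" robot, which carries out instruction objects to seek drop spheres, rotate, or report a spawn location for droppables.
; SeekObject stores a target and calling instruction, then Tick glides and turns the robot toward it at its BeginPlay height.
; Overlapping the target, by Tick check or front-arm collision, stops seeking and hands it to the instruction to document.
; The construction script pins the robot's Z to a fixed height.
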(event OnComponentBeginOverlap(frontArm)
  (params (OverlappedComponent :type Primitive%20Component%20Object%20Reference) (OtherActor :type Actor%20Object%20Reference) (OtherComp :type Primitive%20Component%20Object%20Reference) (OtherBodyIndex :type Integer) (bFromSweep :type Boolean) (SweepResult :type Hit%20Result%20Structure%20%28by%20ref%29))
  ;[1 1 1] Collision
  (bind _asdrop_sphere (Utilities|Casting|CastToDropSphere OtherActor))
  (if (== _asdrop_sphere (Variables|Default|GetclosestObject))
    (CallFunction|DocumentObject)))

(event Custom|Seek
  (params (ds :type Float%20%28single-precision%29))
  (bind _self self)
  (bind _closestobject (Variables|Default|GetclosestObject))
  (bind _returnvalue (Transformation|GetActorLocation _self))
  (bind _returnvalue_2 (Transformation|GetActorLocation _closestobject))
  (bind _returnvalue_3 (Math|Interpolation|VInterptoConstant _returnvalue _returnvalue_2 ds 1e+02))
  ;[1 1 1] Custom Events
  (Transformation|SetActorLocationAndRotation (Math|Vector|MakeVector (.x _returnvalue_3) (.y _returnvalue_3) (Variables|Default|GetclampZLocation)) (Math|Rotator|MakeRotator 0.0 0.0 (.yaw (Math|Interpolation|RInterpTo (Transformation|GetActorRotation) (Math|Rotator|FindLookatRotation _returnvalue _returnvalue_2) ds 1e+01))) true))

(event Custom|DocumentObject
  ;[1 1 1] Custom Events
  (Variables|Default|SetSeekSphere false)
  (Utilities|IsValid (Variables|Default|GetInstruction)
    (:Is%20Valid
      (Class|InstructionDocumentSphere|ExecuteDocumentationfromBP (Variables|Default|GetInstruction) (Variables|Default|GetclosestObject)) ; We have found it, get rid of it
      (Variables|Default|SetInstruction 0)
      (Variables|Default|SetclosestObject 0))))

(event EventBeginPlay
  (Variables|Default|SetrobotName "Grabber")
  (Variables|Default|SetclampZLocation (.z (Transformation|GetActorLocation))))

(event EventSeekObject
  (params (object :type Actor%20Object%20Reference) (callingInstruction :type Instruction%20Document%20Sphere%20Object%20Reference))
  ;[1 1 1] Implementable Events
  (Variables|Default|SetclosestObject object)
  (Variables|Default|SetInstruction callingInstruction)
  (Variables|Default|SetSeekSphere true))

(event EventTick
  (params (DeltaSeconds :type Float%20%28single-precision%29))
  (if (Variables|Default|GetSeekSphere)
    (Utilities|IsValid (Variables|Default|GetclosestObject)
      (:Is%20Valid
        (CallFunction|Seek DeltaSeconds)
        (bind _array_element (Utilities|Array|ForEachLoopwithBreak (Collision|GetOverlappingActors "/Game/Blueprints/DropSphere.DropSphere_C" :!class /Script/Engine.Actor) :!label _label)
          (:LoopBody
            (if (== _array_element (Variables|Default|GetclosestObject))
              (CallFunction|DocumentObject)
              (goto _label Break))))))))

(event EventGetSpawnLocationforObjects
  (params (callingInstruction :type Instruction%20Drop%20Sphere%20Object%20Reference))
  ;[1 1 1] Implementable Events
  (Class|InstructionDropSphere|SetSpawnLocationforDroppables callingInstruction (Transformation|GetWorldLocation (Variables|Default|GetspawnLocation))) ; Send spawn location to code
)

(event EventRotate
  (params (rotationAmount :type Float%20%28single-precision%29) (instruction :type Instruction%20Rotate%20Object%20Reference))
  ;[1 1 1] Implementable Events
  (bind _returnvalue (Transformation|SetActorRotation (Math|Interpolation|RInterpTo (Transformation|GetActorRotation) (Math|Rotator|MakeRotator 0.0 0.0 (+ (.yaw (Transformation|GetActorRotation)) rotationAmount)) 1.0 5.0)))
  (Class|InstructionRotate|SetComplete instruction _returnvalue))

(fn ConstructionScript
  (bind _returnvalue (Transformation|GetActorLocation))
  (Transformation|SetActorLocation (Math|Vector|MakeVector (.x _returnvalue) (.y _returnvalue) 222.0) false true))